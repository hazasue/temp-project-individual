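; Game mode that runs the score and object-spawning loop, and on BeginPlay shows the main UI and plays music.
; SpawnObjects_Event starts SpawnObj, which repeats while InGame, adding score and waiting two seconds per cycle.
; Each cycle uses chained random rolls to pick a rock, eagle or cherry, cherry being the rarest, and calls that type's spawner, found by GetActorOfClass.
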(event Custom|SpawnObjects_Event
  (Utilities|SpawnObj))

(event EventBeginPlay
  (bind _returnvalue (UserInterface|CreateWidget "/Game/BluePrints/WB_Main_UI.WB_Main_UI_C"))
  (UserInterface|Viewport|AddtoViewport _returnvalue 0)
  (Audio|PlaySound2D "/Game/Sounds/itty-bitty-8-bit-by-kevin-macleod-from-filmmusic-io.itty-bitty-8-bit-by-kevin-macleod-from-filmmusic-io" 1.0 1.0 0.0 0 0))

(event EventTick
  (params (DeltaSeconds :type Float%20%28single-precision%29)))

(fn ConstructionScript)