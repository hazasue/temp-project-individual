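; BP_Character is the 2D flipbook player character, with jump input and per-tick updates active only while the game mode's InGame flag is set.
; PlayAnim picks jump or run flipbooks for the Nuguri form, otherwise the rat flipbook, based on player state.
; UpdateRotation flips facing from horizontal velocity, while GetDamage and Heal forward to the player state.
; The Move axis is empty, and movement and Cherry-spawn nodes are unwired.
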(event EventBeginPlay
  (bind _asgm_game_mode (Utilities|Casting|CastToGM_GameMode (Game|GetGameMode)))
  (Variables|Default|SetAs%20GM%20Game%20Mode _asgm_game_mode)
  (bind _asps_player_state (Utilities|Casting|CastToPS_PlayerState (Game|GetPlayerState 0)))
  (Variables|Default|SetAs%20PS%20Player%20State _asps_player_state))

(event Collision|EventActorBeginOverlap
  (params (OtherActor :type Actor%20Object%20Reference)))

(event EventTick
  (params (DeltaSeconds :type Float%20%28single-precision%29))
  (if (Variables|/Game/BluePrints/GM_GameMode.GM_GameMode_C|GetInGame (Variables|Default|GetAs%20GM%20Game%20Mode))
    (CallFunction|PlayAnim)
    (CallFunction|UpdateRotation)))

(event Input|ActionEvents|InputActionDoJump
  (params (Key :type Key%20Structure :default "None"))
  (:Pressed
    (if (Variables|/Game/BluePrints/GM_GameMode.GM_GameMode_C|GetInGame (Variables|Default|GetAs%20GM%20Game%20Mode))
      (Character|Jump)))
  (:Released
    (if (Variables|/Game/BluePrints/GM_GameMode.GM_GameMode_C|GetInGame (Variables|Default|GetAs%20GM%20Game%20Mode))
      (Character|StopJumping))))

(event Input|AxisEvents|InputAxisMove
  (params (AxisValue :type Float%20%28single-precision%29)))

(fn ConstructionScript)

(fn PlayAnim
  (if (Variables|/Game/BluePrints/PS_PlayerState.PS_PlayerState_C|GetisNuguri (Variables|Default|GetAs%20PS%20Player%20State))
    (Sprite|SetFlipbook (Variables|Default|GetSprite) (select (AI|Components|NavMovement|IsFalling (Variables|Character|GetCharacterMovement)) "/Game/Anim/Player/PF_Player_jump.PF_Player_jump" "/Game/Anim/Player/PF_Player_Run.PF_Player_Run"))
    (else
      (Sprite|SetFlipbook (Variables|Default|GetSprite) "/Game/Anim/Player/FB_Rat.FB_Rat"))))

(fn UpdateRotation
  (Utilities|IsValid (Pawn|GetController)
    (:Is%20Valid
      (Math|Float|CompareFloat (.X (Math|Vector|BreakVector (Variables|/Script/Engine.MovementComponent|GetVelocity (Variables|Character|GetCharacterMovement)))) 0.0
        (:>
          (Pawn|SetControlRotation (Pawn|GetController) (Math|Rotator|MakeRotator 0.0 0.0 0.0)))
        (:<
          (Pawn|SetControlRotation (Pawn|GetController) (Math|Rotator|MakeRotator 0.0 0.0 1.8e+02)))))))

(fn GetDamage
  (bind _asps_player_state (Utilities|Casting|CastToPS_PlayerState (Game|GetPlayerState 0)))
  (Default|GetDamage _asps_player_state))

(fn Heal
  (bind _asps_player_state (Utilities|Casting|CastToPS_PlayerState (Game|GetPlayerState 0)))
  (Default|Heal _asps_player_state))